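; Level generator actor that builds a tile-grid layout with a cellular automaton in its Construction Script.
; InitializeLevel randomly seeds live cells from a random stream, then Simulation repeatedly applies birth and death thresholds to Moore-neighbor counts, treating out-of-bounds neighbors as alive.
; FillLevel places Cube instances for live cells and Tile instances for dead ones.
; Index-to-2D conversion divides by Height, so it only holds for square grids.
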(event EventActorBeginOverlap
  (params (OtherActor :type Actor%20Object%20Reference)))

(event Input|KeyboardEvents|F)

(fn ConstructionScript
  (CallFunction|InitializeLevel)
  (for _index (range 0 (Variables|Default|GetSimulationStep))
    (bind _newlevel (CallFunction|Simulation))
    (Variables|Default|SetTileType _newlevel))
  (CallFunction|FillLevel))

(fn InitializeLevel
  (bind _width (Variables|Default|GetWidth))
  (bind _height (Variables|Default|GetHeight))
  (bind _returnvalue (* _width _height))
  ;[1 1 1] Set grid size
  (Utilities|Array|Resize (Variables|Default|GetTileType) _returnvalue)
  ;[1 1 1] Assign random value on the grid
  (for _index (range 0 (- _returnvalue 1))
    (if (< (Math|Random|RandomFloatfromStream (Variables|Default|GetRandromStream)) (Variables|Default|GetAlive%20Chance))
      (LocalVariables|SetValue 1)
      (else
        (LocalVariables|SetValue 0)))
    (Utilities|Array|SetArrayElem (Variables|Default|GetTileType) _index (LocalVariables|GetValue))))

(fn Simulation
  (bind _tiletype (Variables|Default|GetTileType))
  (bind _level (LocalVariables|GetLevel))
  (bind _returnvalue (Utilities|Array|Length _tiletype))
  (Utilities|Array|Resize (LocalVariables|GetLevel) _returnvalue)
  (for _index (range 0 (- _returnvalue 1))
    (bind (_x _y) (CallFunction|1DIndexto2D _index))
    (bind _count (CallFunction|CountAliveNeighbors _x _y))
    (if (== (Utilities|Array|Get(acopy) (Variables|Default|GetTileType) _index) 1)
      (if (< _count (Variables|Default|GetMin%20Death))
        (Utilities|Array|SetArrayElem _level _index 0)
        (else
          (Utilities|Array|SetArrayElem _level _index 1)))
      (elif (> _count (Variables|Default|GetMin%20Alive))
        (Utilities|Array|SetArrayElem _level _index 1)
        (else
          (Utilities|Array|SetArrayElem _level _index 0)))))
  (return (LocalVariables|GetLevel)))

(fn CountAliveNeighbors
  (params (X :type Integer) (Y :type Integer))
  (LocalVariables|SetInX X)
  (LocalVariables|SetInY Y)
  (while (< (LocalVariables|GetP) (Utilities|Array|Length (Variables|Default|GetMoore)))
    ;[1 1 1] Get the 1D index
    (bind _position (CallFunction|CheckPosition (+ (LocalVariables|GetInX) (Utilities|Array|Get(acopy) (Variables|Default|GetMoore) (LocalVariables|GetP))) (+ (LocalVariables|GetInY) (Utilities|Array|Get(acopy) (Variables|Default|GetMoore) (+ (LocalVariables|GetP) 1)))))
    ;[1 1 1] Count alive neighbors
    (if (!= _position -1)
      (if (== (Utilities|Array|Get(acopy) (Variables|Default|GetTileType) _position) 1)
        (LocalVariables|SetCountTemp (+ (LocalVariables|GetCountTemp) 1) :!label _label))
      (else
        (goto _label)))
    (LocalVariables|SetP (+ (LocalVariables|GetP) 2)))
  (return (LocalVariables|GetCountTemp)))

(fn CheckPosition
  (params (X :type Integer :default 0) (Y :type Integer :default 0))
  (bind _width (Variables|Default|GetWidth))
  (if (Math|Boolean|ORBoolean (< X 0) (>= X _width) (< Y 0) (>= Y (Variables|Default|GetHeight)))
    (LocalVariables|SetResult -1)
    (else
      (LocalVariables|SetResult (+ (* Y _width) X))))
  (return (LocalVariables|GetResult)))

(fn 1DIndexto2D
  (params (Index :type Integer :default 0))
  (bind _output_get (LocalVariables|SetTempY (/ Index (Variables|Default|GetHeight))))
  (bind _output_get_2 (LocalVariables|SetTempX (- Index (* _output_get (Variables|Default|GetWidth)))))
  (return _output_get_2 _output_get))

(fn FillLevel
  (bind _tilesize (Variables|Default|GetTileSize))
  (for (_array_element _array_index) (Variables|Default|GetTileType)
    (if (== _array_element 0)
      (Components|InstancedStaticMesh|AddInstance (Variables|Default|GetTile) (Math|Conversions|ToTransform(Vector) (Math|Vector|MakeVector (Math|Conversions|ToFloat(Integer) (* (/ _array_index (Variables|Default|GetHeight)) _tilesize)) (Math|Conversions|ToFloat(Integer) (* (Math|Integer|%(Integer) _array_index (Variables|Default|GetWidth)) _tilesize)) 0.0)))
      (else
        (Components|InstancedStaticMesh|AddInstance (Variables|Default|GetCube) (Math|Conversions|ToTransform(Vector) (Math|Vector|MakeVector (Math|Conversions|ToFloat(Integer) (* (/ _array_index (Variables|Default|GetHeight)) _tilesize)) (Math|Conversions|ToFloat(Integer) (* (Math|Integer|%(Integer) _array_index (Variables|Default|GetWidth)) _tilesize)) 0.0)))))))